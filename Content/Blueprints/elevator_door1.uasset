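; Elevator door actor that slides two panels apart when the player enters its trigger box and can send a linked elevator up.
; A timeline drives both cubes in mirrored X offsets, with a delay on its update path reversing it to close them.
; A second box tracks whether the player is inside.
; If so when the timeline finishes, ElevatorUp is called on the Elevator reference after a delay, gated by DoOnce.
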(event `self.Box.OnComponentBeginOverlap`
  (params (OverlappedComponent :type "PrimitiveComponent Object Reference") (OtherActor :type "Actor Object Reference") (OtherComp :type "PrimitiveComponent Object Reference") (OtherBodyIndex :type Integer) (bFromSweep :type Boolean) (SweepResult :type "HitResult Structure (by ref)"))
  (if (== OtherActor (`GameplayStatics.GetPlayerCharacter` 0))
    (bind (_direction _dual_timeline) (`Timeline|Timeline_0` :!label _label)
      (:`Update`
        (`SceneComponent.K2_SetRelativeLocation` (`self.Cube`) (`KismetMathLibrary.MakeVector` _dual_timeline 0.0 116.0) false false)
        (`SceneComponent.K2_SetRelativeLocation` (`self.Cube1`) (`KismetMathLibrary.MakeVector` (* _dual_timeline -1.0) 0.0 116.0) false false)
        (`KismetSystemLibrary.Delay` 3.0)
        (goto _label :!via `Reverse`))
      (:`Finished`
        (if (`self.isInside?`)
          (`KismetSystemLibrary.Delay` 4.0)
          (`/Engine/EditorBlueprintResources/StandardMacros.DoOnce` false
            (:`Completed`
              (`/Game/Blueprints/elevator_level.elevator up` (`|ConvertAsset` (`self.elevator`))))))))))

(event `self.Box.OnComponentEndOverlap`
  (params (OverlappedComponent :type "PrimitiveComponent Object Reference") (OtherActor :type "Actor Object Reference") (OtherComp :type "PrimitiveComponent Object Reference") (OtherBodyIndex :type Integer))
  (if (== OtherActor (`GameplayStatics.GetPlayerCharacter` 0))
    _))

(event `self.Box1.OnComponentBeginOverlap`
  (params (OverlappedComponent :type "PrimitiveComponent Object Reference") (OtherActor :type "Actor Object Reference") (OtherComp :type "PrimitiveComponent Object Reference") (OtherBodyIndex :type Integer) (bFromSweep :type Boolean) (SweepResult :type "HitResult Structure (by ref)"))
  (if (== OtherActor (`GameplayStatics.GetPlayerCharacter` 0))
    (set `self.isInside?` true)))

(event `self.Box1.OnComponentEndOverlap`
  (params (OverlappedComponent :type "PrimitiveComponent Object Reference") (OtherActor :type "Actor Object Reference") (OtherComp :type "PrimitiveComponent Object Reference") (OtherBodyIndex :type Integer))
  (if (== OtherActor (`GameplayStatics.GetPlayerCharacter` 0))
    (set `self.isInside?` false)))

(fn `UserConstructionScript`)