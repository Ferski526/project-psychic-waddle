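; Double door Blueprint that swings its left and right leaves open or closed each time OpenDoor is called.
; The IsDoorClosed flag chooses whether OpenDoorTimeline plays forward to open or reverses to close.
; The timeline's alpha lerps each leaf's relative yaw, negated for the right leaf so the two rotate in opposite directions.
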(event `OpenDoor`
  (if (`self.IsDoorClosed`)
    (set `self.IsDoorClosed` false)
    (bind (_direction _alpha) (`Timeline|OpenDoorTimeline` :!label _label)
      (:`Update`
        (`SceneComponent.K2_SetRelativeRotation` (`self.LeftDoor`) (`KismetMathLibrary.MakeRotator` 0.0 0.0 (`KismetMathLibrary.Lerp` 0.0 70.0 _alpha)) false false)
        (`SceneComponent.K2_SetRelativeRotation` (`self.RightDoor`) (`KismetMathLibrary.MakeRotator` 0.0 0.0 (`KismetMathLibrary.Lerp` 0.0 70.0 (* _alpha -1.0))) false false)))
    (else
      (set `self.IsDoorClosed` true)
      (goto _label :!via `Reverse`))))

(fn `UserConstructionScript`)